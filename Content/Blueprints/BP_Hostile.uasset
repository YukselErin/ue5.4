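; Hostile AI character that punches in melee, reacts to hits through BPCPhysical, crouches in marked areas and has speed presets.
; Punch montages can queue one follow-up and cancel on movement.
; An arm-aligned sphere trace sends melee damage, with a cooldown for repeat hits on one actor.
; Turn-in-place toward a tagged debug actor is unfinished: its trigger logic is disconnected, though Tick still draws facing and target arrows.
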(event `self.ReceiveBeginPlay`
  ; Cache Debug Targets
  (bind _outactors (`GameplayStatics.GetAllActorsWithTag` "DebugAILookAtBall"))
  (set `self.LookTargetLocation` (`|GetArrayItem` _outactors))
  (bind _outactors_2 (`GameplayStatics.GetAllActorsWithTag` "DebugAIRotateToBall"))
  (set `self.RotateToTargetTransform` (`|GetArrayItem` _outactors_2)))

(event `InterruptAttack`
  (`self.StopAnimMontage` "/Game/Animations/Punching_MontageManny.Punching_MontageManny")
  (set `self.AttackOnCooldown` false)
  (set `self.CueAnotherAttack` false))

(event `Rotate`
  (bind (_returnvalue_roll _returnvalue_pitch _returnvalue_yaw) (`KismetMathLibrary.BreakRotator` (`KismetMathLibrary.RInterpTo` (`self.K2_GetActorRotation`) (`KismetMathLibrary.FindLookAtRotation` (.location (`self.GetTransform`)) (`self.K2_GetActorLocation` (`self.RotateToTargetTransform`))) (`GameplayStatics.GetWorldDeltaSeconds`) 0.5)))
  (`self.K2_SetActorRotation` (`KismetMathLibrary.MakeRotator` 0.0 0.0 _returnvalue_yaw))
  (if (< (`KismetMathLibrary.Abs` (.yaw (`KismetMathLibrary.FindRelativeLookAtRotation` (`KismetMathLibrary.MakeTransform` (+ (.location (`self.GetTransform`)) (0.0 0.0 50.0)) (.rotation (`self.GetTransform`)) (.scale (`self.GetTransform`))) (`self.K2_GetActorLocation` (`self.RotateToTargetTransform`))))) 5.0)
    (set `self.IsPlayingTurnAnimation` false)
    (set `self.TurnLeft` false)
    (set `self.TurnRight` false)))

(event `Swing Attack`
  (`self.Replicated SwingAttack`))

(event `Replicated SwingAttack`
  (if (`self.AttackOnCooldown`)
    (set `self.CueAnotherAttack` true)
    (else
      (set `self.AttackOnCooldown` true)
      (`|PlayMontage` (`self.Mesh`) "/Game/Animations/Punching_MontageManny.Punching_MontageManny"
        (:`then`
          (`KismetSystemLibrary.Delay` 1.0)
          (if (> (`KismetMathLibrary.VSize` (`CharacterMovementComponent.GetLastUpdateVelocity` (`self.CharacterMovement`))) 5.0)
            (`self.InterruptAttack`)
            (elif (`self.CueAnotherAttack`)
              (`self.StopAnimMontage` "/Game/Animations/Punching_MontageManny.Punching_MontageManny")
              (set `self.AttackOnCooldown` false)
              (set `self.CueAnotherAttack` false)
              (`self.Swing Attack`)
              (else
                (`self.StopAnimMontage` "/Game/Animations/Punching_MontageManny.Punching_MontageManny")
                (set `self.AttackOnCooldown` false)
                (set `self.CueAnotherAttack` false)))))))))

(event `self.ReceiveTick`
  (params (DeltaSeconds :type "Float (single-precision)"))
  (`|ExecutionSequence`
    (:`then_0`
      (`self.InterruptAttackIfMoving`))
    (:`then_1`
      (`self.TurnInPlaceDebugDraws`))))

(event `/Game/AI/BPI_TakeMeleeDamage.TakeMeleeDamage`
  (params (Hit :type "HitResult Structure") (AttackVector :type "Vector Structure"))
  (`/Game/PhysicalAnimation/BPC_Physical.HitReaction` (`self.BPC_Physical`) Hit (0.0 0.0 0.0)))

(event `/Game/AI/BPI_HostileAI.EnterCrouchArea`
  (`self.Crouch`))

(event `/Game/AI/BPI_HostileAI.ExitCrouchArea`
  (`self.UnCrouch`))

(fn `InterruptAttackIfMoving`
  (if (> (`KismetMathLibrary.VSize` (`CharacterMovementComponent.GetLastUpdateVelocity` (`self.CharacterMovement`))) 5.0)
    (`self.InterruptAttack`)))

(fn `MeleeAttackDetection`
  (bind _mesh (`self.Mesh`))
  (bind _returnvalue_location (`KismetMathLibrary.BreakTransform` (`SkinnedMeshComponent.GetBoneTransform` _mesh "upperarm_r" "RTS_World")))
  (bind _returnvalue_location_2 (`KismetMathLibrary.BreakTransform` (`SkinnedMeshComponent.GetBoneTransform` _mesh "hand_r" "RTS_World")))
  (bind (_outhit _returnvalue) (`KismetSystemLibrary.SphereTraceSingle` :`Start` _returnvalue_location :`End` (+ (* (`KismetMathLibrary.Normal` (- _returnvalue_location_2 _returnvalue_location)) (`self.MeleeRange`)) _returnvalue_location) :`Radius` 10.0 :`TraceChannel` "TraceTypeQuery1" :`DrawTime` 0.1))
  (if _returnvalue
    (bind (_bblockinghit _binitialoverlap _time _distance _location _impactpoint _normal _impactnormal _physmat _hitactor) (`GameplayStatics.BreakHitResult` _outhit))
    (if (== (`self.LastActor`) _hitactor)
      (if (> (`KismetSystemLibrary.GetGameTimeInSeconds`) (+ (`self.AttackCoolDown`) (`self.LastAttackTime`)))
        (set `self.LastAttackTime` (`KismetSystemLibrary.GetGameTimeInSeconds`) :!label _label)
        (set `self.LastActor` _hitactor)
        (message `/Game/AI/BPI_TakeMeleeDamage.TakeMeleeDamage` _hitactor _outhit (0.0 0.0 0.0)))
      (else
        (goto _label)))))

(fn `PlayTurn`
  (params (YawOffset :type "Float (double-precision)"))
  (locals (LocalYawOffset :type "Float (double-precision)"))
  (bind _output_get (set `local.LocalYawOffset` YawOffset))
  (if (< (`KismetMathLibrary.Abs` _output_get) 60.0)
    (return)
    (elif (> (`KismetMathLibrary.Abs` (`local.LocalYawOffset`)) 135.0)
      (set `self.TurnRight` true :!label _label)
      (set `self.IsPlayingTurnAnimation` true :!label _label_2)
      (`self.ResetTurnMontage` 0.0)
      (elif (>= (`local.LocalYawOffset`) 60.0)
        (goto _label)
        (elif (<= (`local.LocalYawOffset`) -60.0)
          (set `self.TurnLeft` true)
          (goto _label_2))))))

(fn `ResetTurnMontage`
  (params (Duration :type "Float (single-precision)")))

(fn `SetSpeed`
  (params (Speed :type "/Game/AI/Enums/E_NPCSpeeds Enum" :default "NewEnumerator0"))
  (returns (SpeedValue :type "Float (double-precision)"))
  (set `CharacterMovementComponent.MaxWalkSpeed` (select `/Game/AI/Enums/E_NPCSpeeds` Speed :`NewEnumerator1` 150.0 :`NewEnumerator2` 400.0 :`NewEnumerator3` 600.0 :!type "Float (single-precision)") (`self.CharacterMovement`))
  (return 0.0))

(fn `TurnInPlaceDebugDraws`
  (bind _capsulecomponent (`self.CapsuleComponent`))
  (bind _returnvalue (`SceneComponent.K2_GetComponentLocation` _capsulecomponent))
  (bind _returnvalue_2 (`SceneComponent.GetForwardVector` _capsulecomponent))
  (bind _returnvalue_3 (`SceneComponent.K2_GetComponentLocation` (`self.CapsuleComponent`)))
  (bind _returnvalue_4 (`KismetMathLibrary.Normal` (- (`self.K2_GetActorLocation` (`self.RotateToTargetTransform`)) (`SceneComponent.K2_GetComponentLocation` (`self.CapsuleComponent`)))))
  (`|ExecutionSequence`
    (:`then_0`
      (`KismetSystemLibrary.DrawDebugCircle` _returnvalue 25.0 24 (struct :`R` 0.989269 :`G` 0.921466 :`B` 1.0 :`A` 1.0) 0.1 1.0 (1.0 0.0 0.0) (0.0 1.0 0.0))
      (`KismetSystemLibrary.DrawDebugArrow` (+ _returnvalue (* _returnvalue_2 (25.0 25.0 25.0))) (+ _returnvalue (* _returnvalue_2 (40.0 40.0 40.0))) 0.0 (struct :`R` 0.984085 :`G` 0.960198 :`B` 1.0 :`A` 1.0) 0.1 1.0))
    (:`then_1`
      (`KismetSystemLibrary.DrawDebugCircle` _returnvalue_3 30.0 24 (struct :`R` 1.0 :`G` 0.943291 :`B` 0.275312 :`A` 1.0) 0.1 1.0 (1.0 0.0 0.0) (0.0 1.0 0.0))
      (`KismetSystemLibrary.DrawDebugArrow` (+ _returnvalue_3 (* _returnvalue_4 (30.0 30.0 30.0))) (+ _returnvalue_3 (* _returnvalue_4 (45.0 45.0 45.0))) 0.0 (struct :`R` 1.0 :`G` 0.983636 :`B` 0.321127 :`A` 1.0) 0.1 1.0))))

(fn `UserConstructionScript`)