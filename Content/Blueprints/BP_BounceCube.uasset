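; Interactable actor whose cube moves along its relative X axis, with each interaction toggling the motion on or off.
; The construction script caches the cube's starting relative location, and a timeline track scaled by Range drives its X offset from there.
; The timeline restarts on finish while Bouncing is set, so switching it off lets the current cycle complete before the cube stops.
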(event `/Game/Blueprints/BPI_Interactable.OnInteract`
  (params (InteractingPlayer :type "Character Object Reference"))
  (bind _output_get (set `self.Bouncing` (not (`self.Bouncing`))))
  (if _output_get
    (bind (_direction _newtrack_0) (`Timeline|Timeline` :!label _label)
      (:`Update`
        (`SceneComponent.K2_SetRelativeLocation` (`self.Cube`) (`KismetMathLibrary.MakeVector` (+ (* (`self.Range`) _newtrack_0) (.x (`self.CubeInitalLocation`))) (.y (`self.CubeInitalLocation`)) (.z (`self.CubeInitalLocation`))) false false))
      (:`Finished`
        (if (`self.Bouncing`)
          (goto _label :!via `PlayFromStart`)
          (else
            (goto _label :!via `Stop`)))))))

(fn `UserConstructionScript`
  (set `self.CubeInitalLocation` (`SceneComponent.RelativeLocation` (`self.Cube`))))