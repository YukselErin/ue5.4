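; BP_Door is an interactable door that swings open and closed on alternate interactions via a FlipFlop.
; On opening, a dot product between the actor's forward vector and the direction to the player picks the swing direction.
; The Swing timeline scales that signed angle to set the door mesh's absolute world yaw, and plays in reverse to close.
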(event `/Game/Blueprints/BPI_Interactable.OnInteract`
  (params (InteractingPlayer :type "Character Object Reference"))
  (`/Engine/EditorBlueprintResources/StandardMacros.FlipFlop`
    (:`A`
      (set `self.DirectionMultplier` (`KismetMathLibrary.SelectFloat` -90.0 90.0 (> (`KismetMathLibrary.Dot_VectorVector` (`self.GetActorForwardVector`) (`KismetMathLibrary.GetDirectionUnitVector` (`self.K2_GetActorLocation`) (`self.K2_GetActorLocation` InteractingPlayer))) 0.0)))
      (bind (_direction _swingopen) (`Timeline|Swing` :!label _label)
        (:`Update`
          (`SceneComponent.K2_SetWorldRotation` (`self.SM_Door`) (`KismetMathLibrary.MakeRotator` 0.0 0.0 (* _swingopen (`self.DirectionMultplier`))) false false))))
    (:`B`
      (goto _label :!via `Reverse`))))

(fn `UserConstructionScript`)