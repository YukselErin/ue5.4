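; BP_LightSwitch is an interactable switch that toggles a linked BP_Lamp and animates its button.
; On interaction it casts the Lamp reference to BP_Lamp and calls Toggle, doing nothing further if the cast fails.
; A PushButton timeline then lerps the Sphere component along relative Z by ButtonRange, from a rest position cached in the construction script.
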(event `/Game/Blueprints/BPI_Interactable.OnInteract`
  (params (InteractingPlayer :type "Character Object Reference"))
  (bind _z (.z (`self.ButtonFirstPos`)))
  (bind _asbp_lamp (cast `/Game/Blueprints/BP_Lamp` (`self.Lamp`)))
  (`/Game/Blueprints/BP_Lamp.Toggle` _asbp_lamp)
  ;[1 1 1] Button Animation
  (bind (_direction _newtrack_0) (`Timeline|PushButton` :!via `PlayFromStart`)
    (:`Update`
      (`SceneComponent.K2_SetRelativeLocation` (`self.Sphere`) (`KismetMathLibrary.MakeVector` (.x (`self.ButtonFirstPos`)) (.y (`self.ButtonFirstPos`)) (`KismetMathLibrary.Lerp` _z (- _z (`self.ButtonRange`)) _newtrack_0)) false false))))

(fn `UserConstructionScript`
  (set `self.ButtonFirstPos` (`SceneComponent.RelativeLocation` (`self.Sphere`))))