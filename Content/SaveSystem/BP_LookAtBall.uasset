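; BP_LookAtBall is a save-system actor that carries a unique ID and can be moved to a supplied location.
; Its construction script fills an empty ID with a new GUID string, leaving any existing ID intact, and GetID returns it.
; The ChangeState event sets the actor's location directly, without sweep or teleport.
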(event `/Game/SaveSystem/BPI_SaveLocation.ChangeState`
  (params (Location :type "Vector Structure"))
  (`self.K2_SetActorLocation` Location))

(event `self.ReceiveEndPlay`
  (params (EndPlayReason :type "EEndPlayReason Enum" :default "Destroyed")))

(fn `GetID`
  (returns (ID :type String))
  (return (`self.ID`)))

(fn `UserConstructionScript`
  (if (`KismetStringLibrary.IsEmpty` (`self.ID`))
    (set `self.ID` (`KismetGuidLibrary.Conv_GuidToString` (`KismetGuidLibrary.NewGuid`)))))