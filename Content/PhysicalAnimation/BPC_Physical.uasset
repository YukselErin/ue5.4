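; Actor component that gives the owner's skeletal mesh physical hit reactions using a Physical Animation component it creates at BeginPlay.
; HitReaction simulates bodies below the root with the HitReact profile, applies an impulse along the hit direction and draws debug output.
; Tick, enabled only during a reaction, fades the physics blend weight over HitReactionTime, then stops simulation.
; Two other events set up a constant half-weight physical animation blend.
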(event `self.ReceiveBeginPlay`
  (bind _returnvalue (`Actor.GetComponentByClass` (`self.GetOwner`) "/Script/Engine.SkeletalMeshComponent"))
  (`|ExecutionSequence`
    (:`then_0`
      (bind _returnvalue_2 (`|AddComponentByClass` (`self.GetOwner`) "/Script/Engine.PhysicalAnimationComponent"))
      (bind _output_get (set `self.PhysicalAnimationComponent` _returnvalue_2))
      (`PhysicalAnimationComponent.SetSkeletalMeshComponent` _output_get _returnvalue)
      (set `self.Mesh` _returnvalue)
      (`self.SetComponentTickEnabled` false))))

(event `TogglePhysicalAnimation`
  (bind _mesh (`self.Mesh`))
  (bind _root (`self.Root`))
  (bind _physicalanimationcomponent (`self.PhysicalAnimationComponent`))
  (`SkeletalMeshComponent.SetAllBodiesBelowSimulatePhysics` _mesh _root true false)
  (`PhysicalAnimationComponent.ApplyPhysicalAnimationProfileBelow` _physicalanimationcomponent "None" "HitReact" true false)
  (`PhysicalAnimationComponent.SetStrengthMultiplyer` _physicalanimationcomponent 1.0)
  (`SkeletalMeshComponent.SetAllBodiesBelowPhysicsBlendWeight` _mesh _root 0.5 false true))

(event `HitReaction`
  (params (Hit :type "HitResult Structure") (AttackVector :type "Vector Structure"))
  (bind (_bblockinghit _binitialoverlap _time _distance _location _impactpoint _normal _impactnormal _physmat _hitactor _hitcomponent _hitbonename) (`GameplayStatics.BreakHitResult` Hit))
  (bind (_bblockinghit_2 _binitialoverlap_2 _time_2 _distance_2 _location_2 _impactpoint_2) (`GameplayStatics.BreakHitResult` Hit))
  (bind _mesh (`self.Mesh`))
  (bind _returnvalue (select `bool` (== _hitbonename (`self.Root`)) :`false` _hitbonename :`true` (`self.RootFallback`)))
  (bind _attackvector (`self.GetVectorFromHit` Hit))
  (set `self.HitReactionRemainingTime` (`self.HitReactionTime`))
  (`PhysicalAnimationComponent.ApplyPhysicalAnimationProfileBelow` (`self.PhysicalAnimationComponent`) (`self.Root`) "HitReact" true false)
  (`SkeletalMeshComponent.SetAllBodiesBelowSimulatePhysics` _mesh (`self.Root`) true false)
  (bind _returnvalue_2 (* _attackvector (`self.HitForce`)))
  (`PrimitiveComponent.AddImpulse` _mesh _returnvalue_2 _returnvalue true)
  (`KismetSystemLibrary.DrawDebugArrow` _impactpoint_2 (+ _impactpoint_2 _attackvector) 5.0 (struct :`R` 0.366757 :`G` 0.281084 :`B` 1.0 :`A` 1.0) 10.0)
  (`KismetSystemLibrary.PrintString` (`KismetStringLibrary.Conv_NameToString` _returnvalue))
  (`KismetSystemLibrary.PrintString` (`KismetStringLibrary.Conv_DoubleToString` (`KismetMathLibrary.VSize` _returnvalue_2)))
  (`self.SetComponentTickEnabled` true))

(event `CustomEventBound`
  (bind _physicalanimationcomponent (`self.PhysicalAnimationComponent`))
  (bind _mesh (`self.Mesh`))
  (bind _root (`self.Root`))
  (`SkeletalMeshComponent.SetAllBodiesBelowSimulatePhysics` _mesh _root true false)
  (`PhysicalAnimationComponent.ApplyPhysicalAnimationProfileBelow` _physicalanimationcomponent "None" "HitReact" true false)
  (`PhysicalAnimationComponent.SetStrengthMultiplyer` _physicalanimationcomponent 1.0)
  (`SkeletalMeshComponent.SetAllBodiesBelowPhysicsBlendWeight` _mesh _root 0.5 false true))

(event `self.ReceiveTick`
  (params (DeltaSeconds :type "Float (single-precision)"))
  (bind _output_get (set `self.HitReactionRemainingTime` (- (`self.HitReactionRemainingTime`) DeltaSeconds)))
  (if (<= _output_get 0.0)
    (set `self.HitReactionRemainingTime` 0.0)
    (`SkeletalMeshComponent.SetAllBodiesBelowSimulatePhysics` (`self.Mesh`) (`self.Root`) false true)
    (`self.SetComponentTickEnabled` false)
    (else
      (`SkeletalMeshComponent.SetAllBodiesBelowPhysicsBlendWeight` (`self.Mesh`) (`self.Root`) (/ (`self.HitReactionRemainingTime`) (`self.HitReactionTime`)) false true))))

(fn `GetVectorFromHit`
  (params (Hit :type "HitResult Structure"))
  (returns (AttackVector :type "Vector Structure"))
  (bind (_bblockinghit _binitialoverlap _time _distance _location _impactpoint _normal _impactnormal _physmat _hitactor _hitcomponent _hitbonename _bonename _hititem _elementindex _faceindex _tracestart _traceend) (`GameplayStatics.BreakHitResult` Hit))
  (bind _returnvalue (- _traceend _tracestart))
  (if (> (`KismetMathLibrary.VSize` _returnvalue) 0.0)
    (return (`KismetMathLibrary.Normal` _returnvalue))
    (else
      (return (`KismetMathLibrary.Normal` (- _impactpoint _location))))))